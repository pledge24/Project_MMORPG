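; BP_Player is the player character Blueprint with modular, swappable equipment meshes and a nickname widget.
; The construction script makes the five armor parts follow the main Mesh pose as leader.
; ChangeMesh looks up the item's DT_Item row by template ID, blocking-loads its soft mesh references and applies them to the slot's armor or weapon component; IDs of zero or less unequip.
; SetName pushes a name into the nickname widget.
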(event `self.ChangeMesh`
  (params (SlotId :type Integer) (TemplateId :type Integer))
  (bind _skeletal_mesh_ptr (`self.Skeletal Mesh Ptr`))
  ;[1 1 1] 템플릿 id(아이템 id)가 0이하라면 해당 부위 장비를 벗는것으로 간주
  (if (> TemplateId 0)
    (bind _returnvalue (`|GetDataTableRow` "/Game/Gamedata/DT_Item.DT_Item" (`KismetStringLibrary.Conv_StringToName` (`KismetStringLibrary.Conv_IntToString` TemplateId)))
      (:`then`
        (bind (_name _templateid _itemname _itemtype _itemsubtype _levelrequirement _classrequirement _buyprice _sellprice _sellable _maxstack _cooldown _description _icon _hprestore _mprestore _physicalattack _magicalattack _hp _mp _hpregenerate _mpregenerate _skeletalmesh _staticmesh) (break `ItemData` _returnvalue))
        (`self.Load and Set SK Mesh` _skeletalmesh)
        (`self.Load And Set ST Mesh` _staticmesh)))
    (else
      (set `self.Skeletal Mesh Ptr` null)
      (set `self.Static Mesh Ptr` null)))
  (switch `int` SlotId
    (:`1`
      (`SkeletalMeshComponent.SetSkeletalMeshAsset` (`self.Helmet`) _skeletal_mesh_ptr))
    (:`2`
      (`SkeletalMeshComponent.SetSkeletalMeshAsset` (`self.Chest`) _skeletal_mesh_ptr))
    (:`3`
      (`SkeletalMeshComponent.SetSkeletalMeshAsset` (`self.Legs`) _skeletal_mesh_ptr))
    (:`4`
      (`SkeletalMeshComponent.SetSkeletalMeshAsset` (`self.Arms`) _skeletal_mesh_ptr))
    (:`5`
      (`SkeletalMeshComponent.SetSkeletalMeshAsset` (`self.Boots`) _skeletal_mesh_ptr))
    (:`6`
      (`StaticMeshComponent.SetStaticMesh` (`self.WeaponMesh`) (`self.Static Mesh Ptr`)))))

(event `self.SetName`
  (params (ObjectName :type "Text (by ref)"))
  (bind _aswbp_ninkname (cast `/Game/Blueprints/UserInterface/InGame/WBP_Ninkname` (`WidgetComponent.GetWidget` (`self.Ninkname`))))
  (`/Game/Blueprints/UserInterface/InGame/WBP_Ninkname.SetObjectName` _aswbp_ninkname ObjectName))

(fn `Load and Set SK Mesh`
  (params (SkeletalMeshPtr :type "SkeletalMesh Soft Object Reference"))
  (if (`KismetSystemLibrary.IsValidSoftObjectReference` SkeletalMeshPtr)
    (bind _returnvalue (`KismetSystemLibrary.LoadAsset_Blocking` SkeletalMeshPtr))
    (bind _asskeletal_mesh (cast `SkeletalMesh` _returnvalue))
    (set `self.Skeletal Mesh Ptr` _asskeletal_mesh)
    (return)
    (else
      (return))))

(fn `Load And Set ST Mesh`
  (params (StaticMeshPtr :type "StaticMesh Soft Object Reference"))
  (if (`KismetSystemLibrary.IsValidSoftObjectReference` StaticMeshPtr)
    (bind _returnvalue (`KismetSystemLibrary.LoadAsset_Blocking` StaticMeshPtr))
    (bind _asstatic_mesh (cast `StaticMesh` _returnvalue))
    (set `self.Static Mesh Ptr` _asstatic_mesh)
    (return)
    (else
      (return))))

(fn `UserConstructionScript`
  (`SkinnedMeshComponent.SetLeaderPoseComponent` (`self.Helmet`) (`self.Mesh`) false false)
  (`SkinnedMeshComponent.SetLeaderPoseComponent` (`self.Chest`) (`self.Mesh`) false false)
  (`SkinnedMeshComponent.SetLeaderPoseComponent` (`self.Arms`) (`self.Mesh`) false false)
  (`SkinnedMeshComponent.SetLeaderPoseComponent` (`self.Legs`) (`self.Mesh`) false false)
  (`SkinnedMeshComponent.SetLeaderPoseComponent` (`self.Boots`) (`self.Mesh`) false false))