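; BP_Shop is a level object that opens the shop UI when the player walks into its collision area.
; It caches the InGamePlayerController on BeginPlay and uses it to toggle the SHOP widget on overlap begin and end.
; A player in battle mode gets a Korean warning to disable it with Tab instead of the shop.
; End overlap closes the widget without checking which actor left.
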(event `self.ReceiveBeginPlay`
  (bind _asin_game_player_controller (cast `InGamePlayerController` (`GameplayStatics.GetPlayerController` 0)))
  (set `self.PlayerController` _asin_game_player_controller))

(event `self.ShopCollision.OnComponentBeginOverlap`
  (params (OverlappedComponent :type "PrimitiveComponent Object Reference") (OtherActor :type "Actor Object Reference") (OtherComp :type "PrimitiveComponent Object Reference") (OtherBodyIndex :type Integer) (bFromSweep :type Boolean) (SweepResult :type "HitResult Structure (by ref)"))
  (bind _asbp_my_player (cast `/Game/Blueprints/Creatures/Player/BP_MyPlayer` OtherActor))
  (if (`P1MyPlayer.bBattleMode` _asbp_my_player)
    (`InGamePlayerController.DisplayWarningText` (`self.PlayerController`) "Tab을 눌러 전투모드를 비활성화해주세요")
    (else
      (`InGamePlayerController.TurnOnWidget` (`self.PlayerController`) "WIDGET_SHOP"))))

(event `self.ShopCollision.OnComponentEndOverlap`
  (params (OverlappedComponent :type "PrimitiveComponent Object Reference") (OtherActor :type "Actor Object Reference") (OtherComp :type "PrimitiveComponent Object Reference") (OtherBodyIndex :type Integer))
  (`InGamePlayerController.TurnOffWidget` (`self.PlayerController`) "WIDGET_SHOP"))

(fn `UserConstructionScript`)