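; BP_MonsterSpawner is a level object that spawns one monster for each row of MonsterDataTable when play begins.
; It loops over the row names and passes each row's TemplateId to SpawnMonster, whose implementation is outside this graph.
; Transforms are built from the row index, forming an evenly spaced diagonal line at fixed height, independent of the spawner's location.
; Debug prints report the row count and any failed lookup.
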(event `self.ReceiveBeginPlay`
  (bind _monsterdatatable (`self.MonsterDataTable`))
  (bind _outrownames (`DataTableFunctionLibrary.GetDataTableRowNames` _monsterdatatable))
  (`KismetSystemLibrary.PrintString` (`KismetStringLibrary.Conv_IntToString` (`KismetArrayLibrary.Array_Length` _outrownames)))
  (for (_array_element _array_index) _outrownames
    (bind _returnvalue (`|GetDataTableRow` _monsterdatatable _array_element)
      (:`then`
        (bind _returnvalue_2 (* _array_index 100))
        (`self.SpawnMonster` (`.TemplateId` (break `MonsterData` _returnvalue)) (`KismetMathLibrary.MakeTransform` (`KismetMathLibrary.MakeVector` (`KismetMathLibrary.Conv_IntToDouble` _returnvalue_2) (`KismetMathLibrary.Conv_IntToDouble` _returnvalue_2) 100.0))))
      (:`RowNotFound`
        (`KismetSystemLibrary.PrintString` "Hello")))))

(fn `UserConstructionScript`)