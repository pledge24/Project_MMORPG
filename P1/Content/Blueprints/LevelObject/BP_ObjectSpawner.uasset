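; BP_ObjectSpawner is a level object with debug-style functions that spawn monsters from MonsterDataTable.
; SpawnAllMonsters loops over every row and passes its TemplateId to SpawnMonster, placing each along a diagonal by row index at a fixed height.
; SpawnMonsterTest spawns only row "5001" at that line's start; both print a placeholder message for missing rows.
; Neither function is triggered within the Blueprint: BeginPlay is empty and both calls, one delayed, are disconnected.
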(event `self.ReceiveBeginPlay`)

(fn `SpawnAllMonsters`
  (bind _monsterdatatable (`self.MonsterDataTable`))
  (bind _outrownames (`DataTableFunctionLibrary.GetDataTableRowNames` _monsterdatatable))
  (for (_array_element _array_index) _outrownames
    (bind _returnvalue (`|GetDataTableRow` _monsterdatatable _array_element)
      (:`then`
        (bind _returnvalue_2 (* _array_index 100))
        (`self.SpawnMonster` (`.TemplateId` (break `MonsterData` _returnvalue)) (`KismetMathLibrary.MakeTransform` (`KismetMathLibrary.MakeVector` (`KismetMathLibrary.Conv_IntToDouble` _returnvalue_2) (`KismetMathLibrary.Conv_IntToDouble` _returnvalue_2) 100.0))))
      (:`RowNotFound`
        (`KismetSystemLibrary.PrintString` "Hello")))))

(fn `SpawnMonster_Test`
  (bind _returnvalue (* 0 100))
  (bind _returnvalue_2 (`|GetDataTableRow` (`self.MonsterDataTable`) "5001")
    (:`then`
      (`self.SpawnMonster` (`.TemplateId` (break `MonsterData` _returnvalue_2)) (`KismetMathLibrary.MakeTransform` (`KismetMathLibrary.MakeVector` (`KismetMathLibrary.Conv_IntToDouble` _returnvalue) (`KismetMathLibrary.Conv_IntToDouble` _returnvalue) 100.0))))
    (:`RowNotFound`
      (`KismetSystemLibrary.PrintString` "Hello"))))

(fn `UserConstructionScript`)