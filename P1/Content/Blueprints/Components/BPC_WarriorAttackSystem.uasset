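; Warrior attack component that plays a looping normal-attack combo from an array of montages on the character mesh.
; Each attack advances the combo index, sets attack and input-lock flags, and relies on montage notifies or completion to re-enable input.
; A retriggerable delay resets the combo after inactivity.
; SPerformNormalAttack plays a supplied combo step only on P1Player owners that are not P1MyPlayer, apparently mirroring remote players' attacks.
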(event `self.ReceiveBeginPlay`
  (set `self.NormalAttacksLen` (`KismetArrayLibrary.Array_Length` (`self.NormalAttacks`))))

(event `self.PerformNormalAttack`
  (`|ExecutionSequence`
    (:`then_0`
      ;[1 1 1] 1. 수행할 다음 콤보 계산
      (bind _result (`/Engine/EditorBlueprintResources/StandardMacros.IncrementInt` (mod (`self.NormalAttackCombo`) (`self.NormalAttacksLen`)))
        (:`  `
          (bind _output_get (set `self.NormalAttackCombo` _result)))))
    (:`then_1`
      ;[1 1 1] 2. 몽타주 재생
      (`|PlayMontage` (`self.CharacterMesh`) (`|GetArrayItem` (`self.NormalAttacks`) (- (`self.NormalAttackCombo`) 1))
        (:`then`
          (set `self.bIsAttacking` true)
          (set `self.bEnableInputAttack` false)
          (`KismetSystemLibrary.RetriggerableDelay` 2.0)
          (`self.Reset Attack Combo`) ; 콤보 초기화
        )
        (:`OnCompleted`
          (set `self.bIsAttacking` false)
          (set `self.bEnableInputAttack` true))
        (:`OnNotifyBegin`
          (set `self.bEnableInputAttack` true))))))

(event `self.S_PerformNormalAttack`
  (params (Combo :type Integer))
  (bind _returnvalue (`self.GetOwner`))
  (cast `P1MyPlayer` _returnvalue
    (:`CastFailed`
      (cast `P1Player` _returnvalue)
      (`|PlayMontage` (`self.CharacterMesh`) (`|GetArrayItem` (`self.NormalAttacks`) (- Combo 1))))))

(event `Reset Attack Combo`
  (set `self.NormalAttackCombo` 0)
  (set `self.bIsAttacking` false)
  (set `self.bEnableInputAttack` true)
  (`KismetSystemLibrary.PrintString` "Reset Combo"))